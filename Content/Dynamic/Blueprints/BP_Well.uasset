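; BP_Well is an interactable well that yields a photo pickup or prop, BP_PhotoThree, when the player has both a bucket and a rope.
; Its Interaction event checks the character's HasBucket and HasRope flags, then spawns the photo at a hard-coded world transform and destroys the well actor.
; A DoOnce with no reset precedes that check, so only the first interaction is evaluated, even if the items are missing.
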(event `/Game/Dynamic/BlueprintInterfaces/BI_Interact.Interaction`
  (params (MainCharacter :type "/Game/Dynamic/Blueprints/FirstPerson/Blueprints/BP_FirstPersonCharacterGood Object Reference"))
  (`/Engine/EditorBlueprintResources/StandardMacros.DoOnce` false
    (:`Completed`
      (if (and (`/Game/Dynamic/Blueprints/FirstPerson/Blueprints/BP_FirstPersonCharacterGood.HasBucket` MainCharacter) (`/Game/Dynamic/Blueprints/FirstPerson/Blueprints/BP_FirstPersonCharacterGood.HasRope` MainCharacter))
        (`|SpawnActorFromClass` "/Game/Dynamic/Blueprints/BP_PhotoThree.BP_PhotoThree_C" (`KismetMathLibrary.MakeTransform` (12900.0 12389.0 130.0) (struct :`Yaw` 160.0)) "Undefined" "MultiplyWithRoot" null null)
        (`self.K2_DestroyActor`)))))

(fn `UserConstructionScript`
  (`parent.UserConstructionScript`))