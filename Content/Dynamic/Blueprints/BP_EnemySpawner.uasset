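; Enemy spawner actor that starts the night phase once the player has collected all five photos.
; On BeginPlay it caches the first-person player character, then Tick polls its photo flags and uses a DoOnce to fire AllPhotosCollected a single time.
; That event spawns six BP_TheCollector actors at fixed offsets around itself at a set height, switches the player to night and disables their teleporting.
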(event `AllPhotosCollected`
  (bind (_returnvalue_x _returnvalue_y) (`KismetMathLibrary.BreakVector` (`self.K2_GetActorLocation`)))
  (bind (_returnvalue_x_2 _returnvalue_y_2) (`KismetMathLibrary.BreakVector` (`self.K2_GetActorLocation`)))
  (bind (_returnvalue_x_3 _returnvalue_y_3) (`KismetMathLibrary.BreakVector` (`self.K2_GetActorLocation`)))
  (bind (_returnvalue_x_4 _returnvalue_y_4) (`KismetMathLibrary.BreakVector` (`self.K2_GetActorLocation`)))
  (bind (_returnvalue_x_5 _returnvalue_y_5) (`KismetMathLibrary.BreakVector` (`self.K2_GetActorLocation`)))
  (bind (_returnvalue_x_6 _returnvalue_y_6) (`KismetMathLibrary.BreakVector` (`self.K2_GetActorLocation`)))
  (bind _maincharacter (`self.MainCharacter`))
  (`|SpawnActorFromClass` "/Game/Dynamic/Blueprints/TheCollector/BP_TheCollector.BP_TheCollector_C" (`KismetMathLibrary.MakeTransform` (`KismetMathLibrary.MakeVector` (- _returnvalue_x 512.0) _returnvalue_y 88.0) (struct)) "Undefined" "MultiplyWithRoot" null null)
  (`|SpawnActorFromClass` "/Game/Dynamic/Blueprints/TheCollector/BP_TheCollector.BP_TheCollector_C" (`KismetMathLibrary.MakeTransform` (`KismetMathLibrary.MakeVector` _returnvalue_x_2 (- _returnvalue_y_2 512.0) 88.0)) "Undefined" "MultiplyWithRoot" null null)
  (`|SpawnActorFromClass` "/Game/Dynamic/Blueprints/TheCollector/BP_TheCollector.BP_TheCollector_C" (`KismetMathLibrary.MakeTransform` (`KismetMathLibrary.MakeVector` (- _returnvalue_x_3 512.0) (- _returnvalue_y_3 512.0) 88.0)) "Undefined" "MultiplyWithRoot" null null)
  (`|SpawnActorFromClass` "/Game/Dynamic/Blueprints/TheCollector/BP_TheCollector.BP_TheCollector_C" (`KismetMathLibrary.MakeTransform` (`KismetMathLibrary.MakeVector` (+ _returnvalue_x_5 512.0) (+ _returnvalue_y_5 512.0) 88.0)) "Undefined" "MultiplyWithRoot" null null)
  (`|SpawnActorFromClass` "/Game/Dynamic/Blueprints/TheCollector/BP_TheCollector.BP_TheCollector_C" (`KismetMathLibrary.MakeTransform` (`KismetMathLibrary.MakeVector` (+ _returnvalue_x_6 512.0) _returnvalue_y_6 88.0)) "Undefined" "MultiplyWithRoot" null null)
  (`|SpawnActorFromClass` "/Game/Dynamic/Blueprints/TheCollector/BP_TheCollector.BP_TheCollector_C" (`KismetMathLibrary.MakeTransform` (`KismetMathLibrary.MakeVector` _returnvalue_x_4 (+ _returnvalue_y_4 512.0) 88.0)) "Undefined" "MultiplyWithRoot" null null)
  (`/Game/Dynamic/Blueprints/FirstPerson/Blueprints/BP_FirstPersonCharacterGood.Change to Night` _maincharacter)
  (set `/Game/Dynamic/Blueprints/FirstPerson/Blueprints/BP_FirstPersonCharacterGood.CanTeleport` false _maincharacter))

(event `self.ReceiveBeginPlay`
  (bind _asbp_first_person_character_good (cast `/Game/Dynamic/Blueprints/FirstPerson/Blueprints/BP_FirstPersonCharacterGood` (`GameplayStatics.GetPlayerCharacter` 0)))
  (set `self.MainCharacter` _asbp_first_person_character_good))

(event `self.ReceiveTick`
  (params (DeltaSeconds :type "Float (single-precision)"))
  (bind _hasphoto (`/Game/Dynamic/Blueprints/FirstPerson/Blueprints/BP_FirstPersonCharacterGood.HasPhoto` (`self.MainCharacter`)))
  (if (and (`|GetArrayItem` _hasphoto) (`|GetArrayItem` _hasphoto 1) (`|GetArrayItem` _hasphoto 2) (`|GetArrayItem` _hasphoto 3) (`|GetArrayItem` _hasphoto 4))
    (`/Engine/EditorBlueprintResources/StandardMacros.DoOnce` false
      (:`Completed`
        (`self.AllPhotosCollected`)))))

(fn `UserConstructionScript`)