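; BP_Photo is a collectible photo actor, one of five selected by PhotoIndex, that the main character picks up through an Interaction event.
; On interaction it flags that index in the character's HasPhoto array and creates a WBP_PhotoPopUp on the viewport.
; The index selects both the image and the caption shown in the pop-up, then the actor destroys itself.
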(event `/Game/Dynamic/BlueprintInterfaces/BI_Interact.Interaction`
  (params (MainCharacter :type "/Game/Dynamic/Blueprints/FirstPerson/Blueprints/BP_FirstPersonCharacterGood Object Reference"))
  (`KismetArrayLibrary.Array_Set` (`/Game/Dynamic/Blueprints/FirstPerson/Blueprints/BP_FirstPersonCharacterGood.HasPhoto` MainCharacter) (`self.PhotoIndex`) true)
  (bind _returnvalue (`|CreateWidget` "/Game/Dynamic/Widgets/WBP_PhotoPopUp.WBP_PhotoPopUp_C" (`GameplayStatics.GetPlayerController` 0)))
  (`UserWidget.AddToViewport` _returnvalue 0)
  (`Image.SetBrush` (`/Game/Dynamic/Widgets/WBP_PhotoPopUp.Photo` _returnvalue) (make `SlateBrush` (struct :`SpecifiedColor` (struct :`R` 1.0 :`G` 1.0 :`B` 1.0 :`A` 1.0) :`ColorUseRule` "UseColor_Specified") "Image" "NoTile" "NoMirror" (struct :`X` 32.0 :`Y` 32.0) (struct) (select `int` (`self.PhotoIndex`) :`0` "/Game/Static/2DAssets/Photos/PhotoOne.PhotoOne" :`1` "/Game/Static/2DAssets/Photos/PhotoTwo.PhotoTwo" :`2` "/Game/Static/2DAssets/Photos/PhotoThree.PhotoThree" :`3` "/Game/Static/2DAssets/Photos/PhotoFour.PhotoFour" :`4` "/Game/Static/2DAssets/Photos/PhotoFive.PhotoFive" :!type "Object Object Reference")))
  (set `TextBlock.Text` (select `int` (`self.PhotoIndex`) :`0` "Photo One" :`1` "Photo Two" :`2` "Photo Three" :`3` "Photo Four" :`4` "Photo Five" :!type "Text") (`/Game/Dynamic/Widgets/WBP_PhotoPopUp.Dialogue` _returnvalue))
  (`self.K2_DestroyActor`))

(fn `UserConstructionScript`
  (`parent.UserConstructionScript`))