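; BP_Car is an interactable car that serves as the level's exit once the player has collected all five photos.
; Its Interaction event checks the five HasPhoto flags on the main character and, if all are set, opens the main menu map through a DoOnce.
; Otherwise it creates a WBP_Dialogue widget with a line saying it is not yet time and something must be remembered.
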(event `/Game/Dynamic/BlueprintInterfaces/BI_Interact.Interaction`
  (params (MainCharacter :type "/Game/Dynamic/Blueprints/FirstPerson/Blueprints/BP_FirstPersonCharacterGood Object Reference"))
  (bind _hasphoto (`/Game/Dynamic/Blueprints/FirstPerson/Blueprints/BP_FirstPersonCharacterGood.HasPhoto` MainCharacter))
  (if (and (`|GetArrayItem` _hasphoto) (`|GetArrayItem` _hasphoto 1) (`|GetArrayItem` _hasphoto 2) (`|GetArrayItem` _hasphoto 3) (`|GetArrayItem` _hasphoto 4))
    (`/Engine/EditorBlueprintResources/StandardMacros.DoOnce` false
      (:`Completed`
        (`GameplayStatics.OpenLevel` "MAP_MainMenu")))
    (else
      (bind _returnvalue (`|CreateWidget` "/Game/Dynamic/Widgets/WBP_Dialogue.WBP_Dialogue_C" (`GameplayStatics.GetPlayerController` 0)))
      (`UserWidget.AddToViewport` _returnvalue 0)
      (set `TextBlock.Text` "It's still not the time! I have to remember something." (`/Game/Dynamic/Widgets/WBP_Dialogue.DialogueTEXT` _returnvalue)))))

(fn `UserConstructionScript`
  (`parent.UserConstructionScript`))